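; Controller for the fourth VR puzzle (Enigma4), combining three crystal spots with rings of three inner and six outer runes.
; On BeginPlay it links runes to their ring neighbours, binds change events and initializes crystal spots with a shared piece list.
; Rune changes trigger the win check, requiring all crystals and inner runes complete; the outer rune check is bypassed.
; A sphere overlap toggles the VR character's right-hand widget-interaction debug display.
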(event OnComponentBeginOverlap(Sphere)
  (params (OverlappedComponent :type Primitive%20Component%20Object%20Reference) (OtherActor :type Actor%20Object%20Reference) (OtherComp :type Primitive%20Component%20Object%20Reference) (OtherBodyIndex :type Integer) (bFromSweep :type Boolean) (SweepResult :type Hit%20Result%20Structure%20%28by%20ref%29))
  (bind _asbp_vrcharacter (Utilities|Casting|CastToBP_VRCharacter OtherActor))
  (Variables|/Script/UMG.WidgetInteractionComponent|SetbShowDebug (Variables|/Game/_project/BP/BP_VRCharacter.BP_VRCharacter_C|GetWidgetInteractionRight _asbp_vrcharacter) true))

(event OnComponentEndOverlap(Sphere)
  (params (OverlappedComponent :type Primitive%20Component%20Object%20Reference) (OtherActor :type Actor%20Object%20Reference) (OtherComp :type Primitive%20Component%20Object%20Reference) (OtherBodyIndex :type Integer))
  (bind _asbp_vrcharacter (Utilities|Casting|CastToBP_VRCharacter OtherActor))
  (Variables|/Script/UMG.WidgetInteractionComponent|SetbShowDebug (Variables|/Game/_project/BP/BP_VRCharacter.BP_VRCharacter_C|GetWidgetInteractionRight _asbp_vrcharacter) false))

(event Custom|CE_OnCrystalCompleted
  (bind _result (Math|Integer|IncrementInt (Variables|Default|GetCompletedCrystals))
    (:%20%20
      (if (>= _result 3)
        (CallFunction|CEonCrystalsCompleted)))))

(event Custom|CE_OnCrystalsCompleted
  (Variables|Default|SetCrystalsCompleted true))

(event Custom|CE_OnRuneChanged
  (bind _state (CallFunction|CheckforCompletion))
  (if _state
    (CallFunction|CEonEnigma4Completed)))

(event Custom|CE_OnEnigma4Completed
  (Default|CallEnigma4Completed))

(event EventBeginPlay
  (Utilities|FlowControl|Sequence
    (:then_0
      (|SetupInnerRunes)
      (|SetupOuterRunes))
    (:then_1
      (|SetupCrystalSpots))))

(event Collision|EventActorBeginOverlap
  (params (OtherActor :type Actor%20Object%20Reference)))

(event EventTick
  (params (DeltaSeconds :type Float%20%28single-precision%29)))

(fn ConstructionScript)

(fn GetInnerRunebyIndex
  (params (Index :type Integer))
  (bind _asbp_enigma_4_rune (Utilities|Casting|CastToBP_Enigma4_Rune (Variables|/Script/Engine.ChildActorComponent|GetChildActor (Utilities|Select :Index Index :Option%200 (Variables|Default|GetBP_Enigma4_Rune) :Option%201 (Variables|Default|GetBP_Enigma4_Rune1) :Option%202 (Variables|Default|GetBP_Enigma4_Rune2)))))
  (return _asbp_enigma_4_rune))

(fn GetOuterRunebyIndex
  (params (Index :type Integer))
  (bind _bp_enigma4_rune7 (Variables|Default|GetBP_Enigma4_Rune7))
  (bind _bp_enigma4_rune6 (Variables|Default|GetBP_Enigma4_Rune6))
  (bind _bp_enigma4_rune5 (Variables|Default|GetBP_Enigma4_Rune5))
  (bind _bp_enigma4_rune3 (Variables|Default|GetBP_Enigma4_Rune3))
  (bind _bp_enigma4_rune4 (Variables|Default|GetBP_Enigma4_Rune4))
  (bind _bp_enigma4_rune8 (Variables|Default|GetBP_Enigma4_Rune8))
  (bind _returnvalue (Utilities|Select :Index Index :Option%200 _bp_enigma4_rune3 :Option%201 _bp_enigma4_rune4 :Option%202 _bp_enigma4_rune5 :Option%203 _bp_enigma4_rune6 :Option%204 _bp_enigma4_rune7 :Option%205 _bp_enigma4_rune8))
  (Development|PrintString (Utilities|GetDisplayName _returnvalue))
  (bind _asbp_enigma_4_rune (Utilities|Casting|CastToBP_Enigma4_Rune (Variables|/Script/Engine.ChildActorComponent|GetChildActor _returnvalue)))
  (return _asbp_enigma_4_rune))

(fn CheckforCompletion
  (if (Variables|Default|GetCrystalsCompleted)
    (for _index (range 0 2)
      (bind _asbp_enigma_4_rune (CallFunction|GetInnerRunebyIndex _index))
      (if (not (Default|IsComplete _asbp_enigma_4_rune))
        (return false)))
    (for _index_2 (range 0 5)
      (bind _asbp_enigma_4_rune_2 (CallFunction|GetOuterRunebyIndex _index_2))
      (if (not true)
        (return false)))
    (return true)
    (else
      (return false))))