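; BP_Enigma4_CrystalSpot is a placement spot for the Enigma4 puzzle that accepts one crystal piece by matching ID.
; CE_Init hides the transparent placeholder mesh and binds to the grab and drop events of every listed piece.
; Grabbing any piece reveals the placeholder until completion.
; Dropping the correct piece inside the Box destroys it, applies the crystal material and completes the spot; other misplaced drops hide the placeholder.
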(event Custom|CE_OnGrabbed
  (params (MotionController :type Motion%20Controller%20Component%20Object%20Reference) (ActorGrabbed :type Actor%20Object%20Reference))
  (if (not (Variables|Default|GetCompleted))
    (Development|SetHiddeninGame (Variables|Debug|GetStaticMeshComponent) false false)))

(event Custom|CE_OnDropped
  (params (ActorDropped :type Actor%20Object%20Reference))
  (|OnDropped ActorDropped))

(event Custom|CE_Init
  (bind _staticmeshcomponent (Variables|Debug|GetStaticMeshComponent))
  (Utilities|FlowControl|DelayUntilNextTick)
  (Development|SetHiddeninGame _staticmeshcomponent true false)
  (Rendering|Material|SetMaterial _staticmeshcomponent 0 (Variables|Default|GetTransparentMat))
  (for _array_element (Variables|Default|GetPiecesList)
    (EventDispatchers|AssignOnGrabbed (Variables|/Game/_project/BP/BP_Enigma4_Piece.BP_Enigma4_Piece_C|GetBP_Grab _array_element) (delegate Custom|CE_OnGrabbed))
    (EventDispatchers|BindEventtoOnDropped (Variables|/Game/_project/BP/BP_Enigma4_Piece.BP_Enigma4_Piece_C|GetBP_Grab _array_element) (delegate Custom|CE_OnDropped))))

(event EventBeginPlay)

(fn ConstructionScript
  (Components|StaticMesh|SetStaticMesh (Variables|Debug|GetStaticMeshComponent) (Variables|Default|GetStaticMesh)))