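; A rune in the Enigma 4 puzzle that trades ID and symbol material with its left or right neighbor through clickable arrow widgets.
; Each swap plays sounds, raises a change notification and checks both IDs against their target.
; Correct runes glow steadily with a Niagara symbol burst, while incorrect ones pulse via a looping emissive timeline.
; An input lock from the puzzle actor blocks swaps, hides arrows and stops incorrect runes' pulsing.
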(event Custom|CE_BindToInputLocker
  (params (BP_Enigma4 :type BP%20Enigma%204%20Object%20Reference))
  (EventDispatchers|BindEventtoOnLockRuneInput BP_Enigma4 (delegate Custom|CE_LockInput)))

(event Custom|CE_OnLeftArrowClicked
  (CallFunction|SwapRunes (Variables|Default|GetLeftRune)))

(event Custom|CE_LockInput
  (params (Lock :type Boolean))
  (bind _state (CallFunction|IsComplete))
  (bind _output_get (Variables|Default|SetIsInputLocked Lock))
  (if (and (not _output_get) (Variables|Default|GetShowArrows))
    (Rendering|SetVisibility (Variables|Default|GetArrow%20Left) true true)
    (Rendering|SetVisibility (Variables|Default|GetArrow%20Right) true false))
  (if (and _output_get (not _state))
    (Utilities|FlowControl|Sequence
      (:then_0
        (CallFunction|StopTimeline))
      (:then_1
        (Rendering|Material|SetScalarParameterValueonMaterials (Variables|Debug|GetStaticMeshComponent) "Emissive Intensity" 0.0)))
    (elif _state
      (CallFunction|CESetCompletedIntensity)
      (else
        (Utilities|FlowControl|DoOnce false :!label _label
          (:Completed
            (bind _intensity (Timeline|Intensity%20Loop PlayFromStart)
              (:Update
                (Rendering|Material|SetScalarParameterValueonMaterials (Variables|Debug|GetStaticMeshComponent) "Emissive Intensity" _intensity))
              (:Finished
                (if (or (Variables|Default|GetIsInputLocked) (CallFunction|IsComplete))
                  (goto _label Reset)
                  (else
                    (Timeline|Intensity%20Loop PlayFromStart)))))))))))

(event Custom|CE_OnRightArrowClicked
  (CallFunction|SwapRunes (Variables|Default|GetRightRune))
  (Development|PrintString "Clicked"))

(event Custom|CE_SetCompletedIntensity
  (Utilities|FlowControl|Sequence
    (:then_0
      (CallFunction|StopTimeline))
    (:then_1
      (Rendering|Material|SetScalarParameterValueonMaterials (Variables|Debug|GetStaticMeshComponent) "Emissive Intensity" 4.0))
    (:then_2
      (Components|Activation|Activate (Variables|Default|GetNS_BurstE4) true))))

(event Custom|StartLoop
  (Components|Activation|Deactivate (Variables|Default|GetNS_BurstE4))
  (Utilities|FlowControl|DoOnce false :!label _label
    (:Completed
      (bind _intensity (Timeline|Intensity%20Loop PlayFromStart)
        (:Update
          (Rendering|Material|SetScalarParameterValueonMaterials (Variables|Debug|GetStaticMeshComponent) "Emissive Intensity" _intensity))
        (:Finished
          (if (or (Variables|Default|GetIsInputLocked) (CallFunction|IsComplete))
            (goto _label Reset)
            (else
              (Timeline|Intensity%20Loop PlayFromStart))))))))

(event Custom|StopTimeline
  (Utilities|FlowControl|Sequence
    (:then_0
      (Utilities|FlowControl|DoOnce false) ; enters at Reset
    )
    (:then_1
      (bind _intensity (Timeline|Intensity%20Loop Stop)
        (:Update
          (Rendering|Material|SetScalarParameterValueonMaterials (Variables|Debug|GetStaticMeshComponent) "Emissive Intensity" _intensity))
        (:Finished
          (if (or (Variables|Default|GetIsInputLocked) (CallFunction|IsComplete))
            (Utilities|FlowControl|DoOnce false) ; enters at Reset
            (else
              (Timeline|Intensity%20Loop PlayFromStart))))))))

(event EventBeginPlay
  (Utilities|FlowControl|Sequence
    (:then_0
      (Rendering|SetVisibility (Variables|Default|GetArrow%20Left) false false)
      (Rendering|SetVisibility (Variables|Default|GetArrow%20Right) false false)
      (CallFunction|SetMaterial (Variables|Default|GetMaterial))
      (Components|Activation|Deactivate (Variables|Default|GetNS_BurstE4)))
    (:then_1
      (bind _aswd_enigma_4_arrow (Utilities|Casting|CastToWD_Enigma4_Arrow (UserInterface|GetWidget (Variables|Default|GetArrow%20Left))))
      (EventDispatchers|AssignOnClicked (Variables|/Game/_project/Widgets/WD_Enigma4_Arrow.WD_Enigma4_Arrow_C|GetButton _aswd_enigma_4_arrow) (delegate Custom|CE_OnLeftArrowClicked))
      (bind _aswd_enigma_4_arrow_2 (Utilities|Casting|CastToWD_Enigma4_Arrow (UserInterface|GetWidget (Variables|Default|GetArrow%20Right))))
      (EventDispatchers|AssignOnClicked (Variables|/Game/_project/Widgets/WD_Enigma4_Arrow.WD_Enigma4_Arrow_C|GetButton _aswd_enigma_4_arrow_2) (delegate Custom|CE_OnRightArrowClicked)))))

(event EventChangeHelpWidgetVisibility
  (params (Show :type Boolean))
  (bind _isinputlocked (Variables|Default|GetIsInputLocked))
  (bind _returnvalue (not _isinputlocked))
  (bind _output_get (Variables|Default|SetShowArrows Show))
  (if _output_get
    (Rendering|SetVisibility (Variables|Default|GetArrow%20Left) _returnvalue false)
    (Rendering|SetVisibility (Variables|Default|GetArrow%20Right) _returnvalue false)
    (else
      (Rendering|SetVisibility (Variables|Default|GetArrow%20Left) false false)
      (Rendering|SetVisibility (Variables|Default|GetArrow%20Right) false false))))

(fn ConstructionScript
  (CallFunction|SetMaterial (Variables|Default|GetMaterial))
  (Class|NiagaraComponent|SetAsset (Variables|Default|GetNS_BurstE4) (Variables|Default|GetNiagaraSystem) true))

(fn SwapRunes
  (params (Rune :type BP%20Enigma%204%20Rune%20Object%20Reference))
  (if (not (Variables|Default|GetIsInputLocked))
    (LocalVariables|SetTempId (Variables|BP_Enigma4_Rune_C|GetRuneId Rune))
    (Variables|BP_Enigma4_Rune_C|SetRuneId Rune (Variables|Default|GetRuneId))
    (Variables|Default|SetRuneId (LocalVariables|GetTempId))
    (LocalVariables|SetTempMat (CallFunction|GetMaterial Rune))
    (CallFunction|SetMaterial Rune (CallFunction|GetMaterial))
    (CallFunction|SetMaterial (LocalVariables|GetTempMat))
    (CallFunction|PlaySound)
    (CallFunction|PlaySound Rune)
    (Default|CallRuneChanged)
    (Utilities|FlowControl|Sequence
      (:then_0
        (if (CallFunction|IsComplete Rune)
          (CallFunction|CESetCompletedIntensity Rune)
          (else
            (CallFunction|StartLoop Rune))))
      (:then_1
        (if (CallFunction|IsComplete)
          (CallFunction|CESetCompletedIntensity)
          (else
            (CallFunction|StartLoop)))))))

(fn GetMaterial
  (return (Rendering|Material|GetMaterial (Variables|Debug|GetStaticMeshComponent) 0)))

(fn SetMaterial
  (params (Material :type Material%20Interface%20Object%20Reference))
  (Rendering|Material|SetMaterial (Variables|Debug|GetStaticMeshComponent) 0 Material)
  (Class|NiagaraComponent|SetVariableMaterial (Variables|Default|GetNS_BurstE4) "SymbolMaterial" (.Value (Utilities|Map|Find (Variables|Default|GetMaterialParticle) Material))))

(fn IsComplete
  (return (Utilities|Enum|Equal(Enum) (Variables|Default|GetRuneId) (Variables|Default|GetRightRuneId))))

(fn PlaySound
  (Audio|Components|Audio|Play (Variables|Default|GetAudio) 0.0))