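; Widget component that shows an input help hint on its owning actor, hidden at BeginPlay and toggled through ChangeHelpWidgetVisibility.
; It shows only if the owner's optional BP_GrabComponent allows grabbing, and that component's grab and drop events hide and reshow it.
; While shown through that toggle, a looping timer keeps it at a scaled, rotation-independent offset from the owner, facing the player camera.
; The timer function still prints a debug string.
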(event Custom|HideWidget
  (params (MotionController :type Motion%20Controller%20Component%20Object%20Reference) (ActorGrabbed :type Actor%20Object%20Reference))
  (Development|SetHiddeninGame true true))

(event Custom|ShowWidget
  (params (ActorDropped :type Actor%20Object%20Reference))
  (Development|SetHiddeninGame false true))

(event EventTick
  (params (DeltaSeconds :type Float%20%28single-precision%29)))

(event EventChangeHelpWidgetVisibility
  (params (Show :type Boolean))
  (bind _canbeshowed (CallFunction|CanbeGrabbed))
  (bind _returnvalue (and Show _canbeshowed))
  (Development|SetHiddeninGame (not _returnvalue) true)
  (if _returnvalue
    (bind _returnvalue_2 (Utilities|Time|SetTimerbyFunctionName 0 "Update Input Widget Rotation" 0.02 true))
    (Variables|Default|SetTimer _returnvalue_2)
    (else
      (Utilities|Time|ClearandInvalidateTimerbyHandle (Variables|Default|GetTimer)))))

(event EventBeginPlay
  (bind _returnvalue (Components|GetOwner))
  (bind _output_get (Variables|Default|SetLocaDiff (* (Variables|Default|GetRelativeLocation) (Transformation|GetActorScale3D _returnvalue))))
  (Transformation|SetWorldLocation (+ _output_get (Transformation|GetActorLocation _returnvalue)) false false)
  (Development|SetHiddeninGame true true)
  (bind _output_get_2 (Variables|Default|SetGrabComponent (Actor|GetComponentbyClass (Components|GetOwner) "/Game/_project/BP/Components/BP_GrabComponent.BP_GrabComponent_C")))
  (Utilities|IsValid _output_get_2
    (:Is%20Valid
      (EventDispatchers|BindEventtoOnGrabbed _output_get_2 (delegate Custom|HideWidget))
      (EventDispatchers|BindEventtoOnDropped _output_get_2 (delegate Custom|ShowWidget)))))

(fn CanbeGrabbed
  (bind _grabcomponent (Variables|Default|GetGrabComponent))
  (Utilities|IsValid _grabcomponent
    (:Is%20Valid
      (return (Variables|/Game/_project/BP/Components/BP_GrabComponent.BP_GrabComponent_C|GetCanBeGrabbed _grabcomponent)))
    (:Is%20Not%20Valid
      ;[1 1 1] Return true if no grabcomponent
      (return true))))

(fn UpdateInputWidgetRotation
  (Transformation|SetWorldLocation (+ (Transformation|GetActorLocation (Components|GetOwner)) (Variables|Default|GetLocaDiff)) false false)
  (Transformation|SetWorldRotation (Math|Rotator|FindLookatRotation (Transformation|GetWorldLocation) (Camera|GetCameraLocation (Game|GetPlayerCameraManager 0))) false false)
  (Development|PrintString "wawawawa"))