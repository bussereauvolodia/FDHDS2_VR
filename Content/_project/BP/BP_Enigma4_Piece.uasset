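; Grabbable physics piece for the Enigma 4 puzzle, built on a static mesh with a BP_Grab component.
; Grabbing turns off its NSFly effect, and dropping turns it back on and zeroes the mesh's world rotation.
; Reset moves the piece to the player pawn's location and clears its linear and angular velocity, while ShouldReset always returns false.
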(event OnGrabbed(BP_Grab)
  (params (MotionController :type Motion%20Controller%20Component%20Object%20Reference) (ActorGrabbed :type Actor%20Object%20Reference))
  (Components|Activation|Deactivate (Variables|Default|GetNS_Fly)))

(event OnDropped(BP_Grab)
  (params (ActorDropped :type Actor%20Object%20Reference))
  (Components|Activation|Activate (Variables|Default|GetNS_Fly) true)
  (Transformation|SetWorldRotation (Variables|Debug|GetStaticMeshComponent) "0, 0, 0" false false))

(event EventReset
  (bind _staticmeshcomponent (Variables|Debug|GetStaticMeshComponent))
  (Transformation|SetActorLocation (Transformation|GetActorLocation (Game|Player|GetPlayerPawn 0)) false false)
  (Physics|SetPhysicsLinearVelocity _staticmeshcomponent "0, 0, 0" false "None")
  (Class|PrimitiveComponent|SetPhysicsAngularVelocityinRadians _staticmeshcomponent "0, 0, 0" false "None"))

(fn ConstructionScript)

(fn ShouldReset
  (return false))