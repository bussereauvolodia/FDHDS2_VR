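; Grabbable symbol cube for a puzzle, turned around its yaw axis by a motion controller to select a symbol.
; While held, a looping timer follows the controller's look-at yaw change and releases the grab beyond MaxDistance.
; On drop, a timeline snaps it to the nearest 90°, looks up the symbol in FixedRotations and calls a completion check if correct.
; Helper functions step the rotation, assign symbols and the solution, lock grabbing and set emissive intensity.
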(event OnGrabbed(BP_GrabComponent)
  (params (MotionController :type Motion%20Controller%20Component%20Object%20Reference) (ActorGrabbed :type Actor%20Object%20Reference))
  (bind _output_get (Variables|Default|SetMotion%20Controller MotionController))
  (Variables|Default|SetLookAtAtGrab (Math|Rotator|FindLookatRotation (Transformation|GetWorldLocation (Variables|Default|GetCube)) (Transformation|GetWorldLocation _output_get)))
  (Variables|Default|SetCubeRotationVar (Variables|/Script/Engine.SceneComponent|GetRelativeRotation (Variables|Default|GetCube)))
  (bind _returnvalue (Utilities|Time|SetTimerbyFunctionName 0 "UpdateRotation" 0.02 true))
  (Variables|Default|SetTimer _returnvalue)
  (Audio|Components|Audio|Play (Variables|Default|GetAudio) 0.0)
  (Development|PrintString "bbbbb")
  (bind _progression (Timeline|Rotation Stop)
    (:Update
      (Transformation|SetRelativeRotation (Variables|Default|GetCube) (Math|Rotator|MakeRotator (.roll (Variables|Default|GetCubeRotationVar)) (.pitch (Variables|Default|GetCubeRotationVar)) (Math|Float|Lerp (.yaw (Variables|Default|GetCubeRotationVar)) (stale OnDropped(BP_GrabComponent) _ztarget) _progression)) false false))
    (:Finished
      (Utilities|FlowControl|Sequence
        (:then_0
          (bind _output_get_2 (Variables|Default|SetCurrentSymbol (CallFunction|GetCurrentSymbol)))
          (Development|PrintString _output_get_2)
          (if (Utilities|Enum|Equal(Enum) (Variables|Default|GetCorrectSymbol) _output_get_2)
            (Default|CallCheckforCompletion)))
        (:then_1
          (Audio|Components|Audio|Stop (Variables|Default|GetAudio)))))))

(event OnDropped(BP_GrabComponent)
  (params (ActorDropped :type Actor%20Object%20Reference))
  (bind _cuberotationvar (Variables|Default|GetCubeRotationVar))
  (Utilities|Time|ClearandInvalidateTimerbyHandle (Variables|Default|GetTimer))
  (Variables|Default|SetMotion%20Controller 0)
  (bind _ztarget (CallFunction|FindClosestPosition (.Yaw (Math|Rotator|BreakRotator (Variables|/Script/Engine.SceneComponent|GetRelativeRotation (Variables|Default|GetCube))))))
  (bind _progression (Timeline|Rotation PlayFromStart)
    (:Update
      (Transformation|SetRelativeRotation (Variables|Default|GetCube) (Math|Rotator|MakeRotator (.roll _cuberotationvar) (.pitch _cuberotationvar) (Math|Float|Lerp (.yaw _cuberotationvar) _ztarget _progression)) false false))
    (:Finished
      (Utilities|FlowControl|Sequence
        (:then_0
          (bind _output_get (Variables|Default|SetCurrentSymbol (CallFunction|GetCurrentSymbol)))
          (Development|PrintString _output_get)
          (if (Utilities|Enum|Equal(Enum) (Variables|Default|GetCorrectSymbol) _output_get)
            (Default|CallCheckforCompletion)))
        (:then_1
          (Audio|Components|Audio|Stop (Variables|Default|GetAudio)))))))

(event EventBeginPlay
  (Audio|Components|Audio|Stop (Variables|Default|GetAudio))
  (CallFunction|SetMaterialIntensity 0.0))

(fn ConstructionScript
  (Rendering|Material|SetMaterial (Variables|Default|GetCube) 0 (Variables|SymbolCubeSetup|GetMaterial%20Instance)))

(fn UpdateRotation
  (bind _motion_controller (Variables|Default|GetMotion%20Controller))
  (bind _cube (Variables|Default|GetCube))
  (bind _cuberotationvar (Variables|Default|GetCubeRotationVar))
  (bind _returnvalue (Transformation|GetWorldLocation _cube))
  (bind _returnvalue_2 (Transformation|GetWorldLocation _motion_controller))
  (if (> (Math|Vector|Distance(Vector) _returnvalue _returnvalue_2) (Variables|Default|GetMaxDistance))
    (Default|TryRelease (Variables|Default|GetBP_GrabComponent))
    (else
      (Transformation|SetRelativeRotation (Variables|Default|GetCube) (Math|Rotator|MakeRotator (.roll _cuberotationvar) (.pitch _cuberotationvar) (+ (.yaw _cuberotationvar) (- (.yaw (Math|Rotator|FindLookatRotation _returnvalue _returnvalue_2)) (.yaw (Variables|Default|GetLookAtAtGrab))))) false false))))

(fn FindClosestPosition
  (params (ZRotation :type Float%20%28double-precision%29))
  (bind _returnvalue (+ ZRotation 3.6e+03))
  (bind _cube (Variables|Default|GetCube))
  (bind _returnvalue_2 (Transformation|GetWorldRotation _cube))
  (bind _returnvalue_3 (Math|Float|%(Float) _returnvalue 3.6e+02))
  (bind _returnvalue_4 (Math|Float|%(Float) _returnvalue_3 9e+01))
  ;[1 1 1] Reset value to in 0-360
  (Transformation|SetRelativeRotation _cube (Math|Rotator|MakeRotator (.roll _returnvalue_2) (.pitch _returnvalue_2) _returnvalue_3) false false)
  (Variables|Default|SetCubeRotationVar (Math|Rotator|MakeRotator (.roll _returnvalue_2) (.pitch _returnvalue_2) _returnvalue_3))
  (return (+ _returnvalue_3 (Math|Float|SelectFloat (* _returnvalue_4 -1.0) (- 9e+01 _returnvalue_4) (< _returnvalue_4 45.0)))))

(fn IsCorrect
  (return (Utilities|Enum|Equal(Enum) (CallFunction|GetCurrentSymbol) (Variables|Default|GetCorrectSymbol))))

(fn LockGrabbing
  (params (Lock :type Boolean))
  (Variables|/Game/_project/BP/Components/BP_GrabComponent.BP_GrabComponent_C|SetCanBeGrabbed (Variables|Default|GetBP_GrabComponent) (not Lock)))

(fn Rotate90°
  (bind _cube (Variables|Default|GetCube))
  (bind _relativerotation (Variables|/Script/Engine.SceneComponent|GetRelativeRotation _cube))
  (bind _ztarget (CallFunction|FindClosestPosition (+ (.yaw (Variables|/Script/Engine.SceneComponent|GetRelativeRotation (Variables|Default|GetCube))) 9e+01)))
  (Transformation|SetRelativeRotation _cube (Math|Rotator|MakeRotator (.roll _relativerotation) (.pitch _relativerotation) (Math|Float|SelectFloat 0.0 _ztarget (== _ztarget 3.6e+02))) false false)
  (Variables|SymbolCubeSetup|SetCurrentSelectedSymbol (CallFunction|GetCurrentSymbol)))

(fn GetCurrentSymbol
  (bind _cube (Variables|Default|GetCube))
  (bind _fixedrotations (Variables|Default|GetFixedRotations))
  (bind _relativerotation (Variables|/Script/Engine.SceneComponent|GetRelativeRotation _cube))
  (bind _returnvalue (== (.yaw _relativerotation) 3.6e+02))
  (bind _returnvalue_2 (Math|Float|SelectFloat 0.0 (.yaw _relativerotation) _returnvalue))
  (bind (_value _returnvalue_3) (Utilities|Map|Find _fixedrotations _returnvalue_2))
  (if _returnvalue_3
    (return _value)
    (else
      (return (Utilities|String|Append "Not Found, Rot : " (Utilities|String|ToString(Float) _returnvalue_2))))))

(fn ChangeCurrentSymbol
  (bind _returnvalue (== 0.0 3.6e+02))
  (bind _fixedrotations (Variables|Default|GetFixedRotations))
  (bind _cube (Variables|Default|GetCube))
  (bind _relativerotation (Variables|/Script/Engine.SceneComponent|GetRelativeRotation _cube))
  (bind _returnvalue_2 (Math|Float|SelectFloat 0.0 (.yaw _relativerotation) _returnvalue))
  (if (.ReturnValue (Utilities|Map|Find _fixedrotations _returnvalue_2))
    (Utilities|Map|Add _fixedrotations _returnvalue_2 (Variables|SymbolCubeSetup|GetCurrentSelectedSymbol))
    (else
      (Development|PrintString (Utilities|String|ToString(Float) _returnvalue_2)))))

(fn SetCurrentSymbolasCorrect
  (Variables|Default|SetCorrectSymbol (Variables|SymbolCubeSetup|GetCurrentSelectedSymbol)))

(fn SetMaterialIntensity
  (params (Intensity :type Float%20%28double-precision%29))
  ;[1 1 1] Si on veut faire allumer les Cubes aussi
  (Rendering|Material|SetScalarParameterValueonMaterials (Variables|Default|GetCube) "Emissive Intensity" Intensity))