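; BP_Enigma3 manages the third puzzle, rewarding completed columns with the piece for Enigma 4.
; It hides Enigma4Piece on BeginPlay, counts OnColumnCompleted events and reveals the piece when the count equals ColumnAmount.
; It also binds to the piece's motion-controller grab component and relays the grab through its own OnPieceGrabbed dispatcher.
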(event Custom|OnColumnCompleted
  (params (Column :type BP%20Column%20Object%20Reference))
  (bind _result (Math|Float|IncrementFloat (Variables|Default|GetCurrentAmount))
    (:%20%20
      (if (== _result (Variables|Default|GetColumnAmount))
        (Rendering|SetActorHiddenInGame (Variables|Default|GetEnigma4%20Piece) false)))))

(event Custom|CE_PieceGrabbed
  (params (MotionController :type Motion%20Controller%20Component%20Object%20Reference) (ActorGrabbed :type Actor%20Object%20Reference))
  (Default|CallOnPieceGrabbed))

(event EventBeginPlay
  (bind _enigma4_piece (Variables|Default|GetEnigma4%20Piece))
  (Variables|Default|SetCurrentAmount 0.0)
  (Rendering|SetActorHiddenInGame _enigma4_piece true)
  (EventDispatchers|BindEventtoOnGrabbed (Variables|/Game/_project/BP/BP_Enigma4_Piece.BP_Enigma4_Piece_C|GetBP_Grab _enigma4_piece) (delegate Custom|CE_PieceGrabbed)))

(fn ConstructionScript)