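; BP_Column is a puzzle pillar in Enigma 3, completed when its three attached symbol cubes are all correct.
; Cubes stay grab-locked until every PreviousColumn completes, then WallWord enables and a looping timeline pulses pillar and cube emissive.
; Completion locks the cubes, fixes the glow, broadcasts OnCompletion and notifies EndingPlace, firing a Niagara beam and audio toward it until its piece is grabbed.
; CreateSymbolCubes spawns the cubes at placeholder transforms.
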(event Custom|Create%20Symbol%20Cubes
  (bind _self self)
  (if (Utilities|Array|IsEmpty (Variables|Default|GetSymbolCubes))
    (for _index (range 0 2)
      (bind _returnvalue (Game|SpawnActorfromClass "/Game/_project/BP/Enigma3/BP_SymbolCube.BP_SymbolCube_C" (Math|Transform|MakeTransform (.location (Transformation|GetWorldTransform (Utilities|Select :Index _index :Option%200 (Variables|Default|GetCube1) :Option%201 (Variables|Default|GetCube2) :Option%202 (Variables|Default|GetCube3)))) "0, 0, 0" (.scale (Transformation|GetWorldTransform (Utilities|Select :Index _index :Option%200 (Variables|Default|GetCube1) :Option%201 (Variables|Default|GetCube2) :Option%202 (Variables|Default|GetCube3))))) "Undefined" "MultiplyWithRoot" _self 0))
      (Utilities|Array|Add (Variables|Default|GetSymbolCubes) _returnvalue)
      (Transformation|AttachActorToActor _returnvalue _self "None" "KeepWorld" "KeepWorld" "KeepWorld" true))))

(event Custom|CheckForCompletion
  (bind _endingplace (Variables|Default|GetEndingPlace))
  (if (CallFunction|AreAllCubesCompleted)
    (Utilities|FlowControl|Sequence
      (:then_0
        (Variables|Default|SetCurrentState "NewEnumerator2")
        (Default|CallOnCompletion)
        (for _array_element (Variables|Default|GetSymbolCubes)
          (Default|LockGrabbing _array_element true))
        (Utilities|IsValid _endingplace
          (:Is%20Valid
            (Default|OnColumnCompleted _endingplace self))))
      (:then_1
        (bind _intensity (Timeline|IntensityLoop Stop)
          (:Update
            (Rendering|Material|SetScalarParameterValueonMaterials (Variables|Default|GetPillarMesh) "Emissive Intensity" _intensity)
            ;[1 1 1] Si Symbol Cubes update intensity aussi
            (for _array_element_2 (Variables|Default|GetSymbolCubes)
              (Default|SetMaterialIntensity _array_element_2 _intensity)))
          (:Finished
            (if (Utilities|Enum|Equal(Enum) (Variables|Default|GetCurrentState) "NewEnumerator1")
              (Timeline|IntensityLoop PlayFromStart)))))
      (:then_2
        (Rendering|Material|SetScalarParameterValueonMaterials (Variables|Default|GetPillarMesh) "Emissive Intensity" 4.0)
        (Default|SetEnabled (Variables|Default|GetWallWord) false)
        (for _array_element_3 (Variables|Default|GetSymbolCubes)
          (Default|SetMaterialIntensity _array_element_3 0.0)))
      (:then_3
        (Utilities|IsValid (Variables|Default|GetEndingPlace)
          (:Is%20Valid
            (Components|Activation|Activate (Variables|Default|GetNS_Beam) false)
            (Audio|Components|Audio|Play (Variables|Default|GetAudio) 0.0)))))))

(event Custom|CE_DeactivateBeam
  (Components|Activation|Deactivate (Variables|Default|GetNS_Beam)))

(event Custom|ActiveIntensityLoop
  (if (Utilities|Enum|Equal(Enum) (Variables|Default|GetCurrentState) "NewEnumerator1") :!label _label
    (bind _intensity (Timeline|IntensityLoop PlayFromStart)
      (:Update
        (Rendering|Material|SetScalarParameterValueonMaterials (Variables|Default|GetPillarMesh) "Emissive Intensity" _intensity)
        ;[1 1 1] Si Symbol Cubes update intensity aussi
        (for _array_element (Variables|Default|GetSymbolCubes)
          (Default|SetMaterialIntensity _array_element _intensity)))
      (:Finished
        (goto _label)))))

(event EventBeginPlay
  (bind _result (CallFunction|AreAllPreviousColumnsCompleted))
  (bind _ns_beam (Variables|Default|GetNS_Beam))
  (bind _endingplace (Variables|Default|GetEndingPlace))
  (Utilities|IsValid _endingplace
    (:Is%20Valid
      (EventDispatchers|BindEventtoOnPieceGrabbed _endingplace (delegate Custom|CE_DeactivateBeam))
      (Effects|Components|ParticleSystem|SetVectorParameter _ns_beam "User.EndBeamPosition" (Transformation|GetActorLocation _endingplace)))
    (:Is%20Not%20Valid
      _))
  (Components|Activation|Deactivate _ns_beam)
  (for _array_element (Variables|Default|GetSymbolCubes)
    (EventDispatchers|BindEventtoCheckforCompletion _array_element (EventDispatchers|CreateEvent :!event Custom|CheckForCompletion))
    (Default|LockGrabbing _array_element (not _result)))
  (if _result
    (Variables|Default|SetCurrentState "NewEnumerator1")
    (CallFunction|ActiveIntensityLoop)
    (Default|SetEnabled (Variables|Default|GetWallWord) true)
    (else
      (for _array_element_2 (Variables|Default|GetPreviousColumn)
        (EventDispatchers|BindEventtoOnCompletion _array_element_2 (EventDispatchers|CreateEvent :!event TryUnlockColumn))))))

(fn ConstructionScript)

(fn AreAllCubesCompleted
  (for _array_element (Variables|Default|GetSymbolCubes)
    (if (not (Default|IsCorrect _array_element))
      (return false)))
  (return true))

(fn TryUnlockColumn
  (if (CallFunction|AreAllPreviousColumnsCompleted)
    (for _array_element (Variables|Default|GetSymbolCubes)
      (Default|LockGrabbing _array_element false))
    (Variables|Default|SetCurrentState "NewEnumerator1")
    (CallFunction|ActiveIntensityLoop)
    (Default|SetEnabled (Variables|Default|GetWallWord) true)))

(fn AreAllPreviousColumnsCompleted
  (for _array_element (Variables|Default|GetPreviousColumn)
    (if (not (Utilities|Enum|Equal(Enum) (Variables|BP_Column_C|GetCurrentState _array_element) "NewEnumerator2"))
      (return false)))
  (return true))