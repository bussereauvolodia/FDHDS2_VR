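; BP_Enigma1 is the controller for the first puzzle, which is solved when all of its pillars are completed.
; On BeginPlay it hides its static mesh and binds to each pillar's OnCompleted delegate.
; Each completion event rechecks every pillar.
; Once all pass, it locks their current pieces, deactivates the level 1 particles, destroys the invisible mesh and prints a completion message.
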(event Custom|CE_OnCompleted
  (if (CallFunction|AreAllPillarsCompleted)
    (CallFunction|CEonEnigmaComplete)))

(event Custom|CE_OnEnigmaComplete
  ;[1 1 1] On Enigma completed logic
  (for _array_element (Variables|Default|GetPillars)
    (Default|CELockCurrentPiece _array_element))
  (Components|Activation|Deactivate (Variables|Default|GetLvl1_Particules))
  (Components|DestroyComponent (Variables|Default|GetStaticMesh))
  (Development|PrintString "Enigma 1 Completed !!!!" true true "(R=0.000000,G=0.660000,B=1.000000,A=1.000000)" 5.0))

(event EventBeginPlay
  (Rendering|SetVisibility (Variables|Default|GetStaticMesh) false false)
  (for _array_element (Variables|Default|GetPillars)
    (EventDispatchers|AssignOnCompleted _array_element (EventDispatchers|CreateEvent :!event Custom|CE_OnCompleted))))

(fn ConstructionScript)

(fn AreAllPillarsCompleted
  (for _array_element (Variables|Default|GetPillars)
    (if (not (Default|IsCompleted _array_element))
      (return false)))
  (return true))