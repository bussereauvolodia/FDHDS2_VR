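; Puzzle pillar that accepts one correct piece from a list of grabbable pieces and signals completion when it is placed.
; While unoccupied, grabbing any listed piece reveals an overlay of the right piece's mesh.
; On drop over the pillar, the right piece snaps to the overlay's transform with sound and Niagara feedback, while others only play an error sound.
; A separate event can lock the placed piece against grabbing.
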(event Custom|CE_LockCurrentPiece
  (bind _placedpiece (Variables|Default|GetPlacedPiece))
  (Utilities|IsValid _placedpiece
    (:Is%20Valid
      (Variables|/Game/_project/BP/Components/BP_GrabComponent.BP_GrabComponent_C|SetCanBeGrabbed (Variables|/Game/_project/BP/Enigma1/BP_RuinPiece.BP_RuinPiece_C|GetBP_GrabComponent _placedpiece) false))))

(event Custom|CE_OnGrabbed
  (params (MotionController :type Motion%20Controller%20Component%20Object%20Reference) (ActorGrabbed :type Actor%20Object%20Reference))
  (Utilities|FlowControl|Sequence
    (:then_0
      (if (== (Variables|Default|GetPlacedPiece) ActorGrabbed)
        (Variables|Default|SetPlacedPiece 0)))
    (:then_1
      (if (not (CallFunction|IsOccupied))
        (CallFunction|SetupPieceOverlay (Variables|Default|GetRightPiece))
        (Development|SetHiddeninGame (Variables|Default|GetPieceOverlay) false false)))))

(event Custom|CE_PlacePiece
  (params (PieceDropped :type Actor%20Object%20Reference))
  (bind _ruinpiece (CallFunction|GetPiecefromList PieceDropped))
  (bind _rightpiece (Variables|Default|GetRightPiece))
  (bind _returnvalue (== _rightpiece PieceDropped))
  (if (Collision|IsOverlappingActor PieceDropped self :!class /Script/Engine.Actor)
    (Transformation|SetActorLocation PieceDropped (Transformation|GetWorldLocation (Variables|Default|GetPieceOverlay)) false true)
    (Transformation|SetActorRotation PieceDropped (Transformation|GetWorldRotation (Variables|Default|GetPieceOverlay)) true)
    (Utilities|IsValid _ruinpiece
      (:Is%20Valid
        (bind _output_get (Variables|Default|SetPlacedPiece _ruinpiece))
        (Default|OnPlaced _output_get _returnvalue)
        (if _returnvalue
          (Audio|Components|Audio|Play (Variables|Default|GetAudio) 0.0)
          (Components|Activation|Activate (Variables|Default|GetNS_GoodEffect) true)
          (Audio|PlaySoundatLocation "/Game/_project/Assets/Audio/humordome-fairy-sparkle-451414.humordome-fairy-sparkle-451414" (Transformation|GetActorLocation) "0, 0, 0" 1.0 1.0 0.0 0 0 0 0)
          (Default|CallOnCompleted))))))

(event Custom|CE_OnDropped
  (params (ActorDropped :type Actor%20Object%20Reference))
  (if (not (CallFunction|IsOccupied))
    (Development|SetHiddeninGame (Variables|Default|GetPieceOverlay) true false)
    (if (Collision|IsOverlappingActor ActorDropped self :!class /Script/Engine.Actor)
      (if (== ActorDropped (Variables|Default|GetRightPiece))
        (CallFunction|CEPlacePiece ActorDropped)
        (else
          (Audio|PlaySoundatLocation "/Game/_project/Assets/Audio/PieceImpossiblePlacer.PieceImpossiblePlacer" (Transformation|GetActorLocation) "0, 0, 0" 1.0 1.0 0.0 0 0 0 0))))))

(event EventBeginPlay
  (Development|SetHiddeninGame (Variables|Default|GetPieceOverlay) true false)
  (for _array_element (Variables|Default|GetPiecesList)
    (EventDispatchers|BindEventtoOnGrabbed (Variables|/Game/_project/BP/Enigma1/BP_RuinPiece.BP_RuinPiece_C|GetBP_GrabComponent _array_element) (EventDispatchers|CreateEvent :!event Custom|CE_OnGrabbed))
    (EventDispatchers|BindEventtoOnDropped (Variables|/Game/_project/BP/Enigma1/BP_RuinPiece.BP_RuinPiece_C|GetBP_GrabComponent _array_element) (EventDispatchers|CreateEvent :!event Custom|CE_OnDropped))))

(fn ConstructionScript
  (bind _rightpiece (Variables|Default|GetRightPiece))
  (bind _pieceoverlay (Variables|Default|GetPieceOverlay))
  (Components|StaticMesh|SetStaticMesh _pieceoverlay (Variables|/Game/_project/BP/Enigma1/BP_RuinPiece.BP_RuinPiece_C|GetMesh _rightpiece))
  (Transformation|SetWorldScale3D _pieceoverlay (Transformation|GetActorScale3D _rightpiece)))

(fn SetupPieceOverlay
  (params (ActorGrabbed :type Actor%20Object%20Reference))
  (bind _ruinpiece (CallFunction|GetPiecefromList ActorGrabbed))
  (bind _pieceoverlay (Variables|Default|GetPieceOverlay))
  (Utilities|IsValid _ruinpiece
    (:Is%20Valid
      (LocalVariables|SetFound true)
      (Components|StaticMesh|SetStaticMesh _pieceoverlay (Variables|/Game/_project/BP/Enigma1/BP_RuinPiece.BP_RuinPiece_C|GetMesh _ruinpiece))
      (Transformation|SetWorldScale3D _pieceoverlay (Transformation|GetActorScale3D _ruinpiece)))
    (:Is%20Not%20Valid
      (return false))))

(fn GetPiecefromList
  (params (Actor :type Actor%20Object%20Reference))
  (for _array_element (Variables|Default|GetPiecesList)
    (if (== _array_element Actor)
      (return _array_element)))
  (return 0))

(fn IsCompleted
  (Utilities|IsValid (Variables|Default|GetPlacedPiece)
    (:Is%20Valid
      (return (== (Variables|Default|GetPlacedPiece) (Variables|Default|GetRightPiece))))
    (:Is%20Not%20Valid
      (return false))))

(fn IsOccupied
  (return (Utilities|IsValid (Variables|Default|GetPlacedPiece))))