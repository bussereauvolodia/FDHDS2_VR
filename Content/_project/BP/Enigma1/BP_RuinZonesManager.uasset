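; BP_RuinZonesManager is a manager for the Enigma1 ruin puzzle that resets watched pieces when they leave all zones.
; GetPieceFromList searches PieceList for a given actor, and IsWatchedPiece uses it to report whether that actor is tracked.
; ActorLeftAllZones calls CEReset on the matching piece from inside a debug "Hello" print loop, repeating the reset each iteration and again on completion.
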(event EventActorLeftAllZones
  (params (Actor :type Actor%20Object%20Reference))
  (for _index (range 0 100)
    (Development|PrintString "Hello")
    (Default|CEReset (CallFunction|GetPiecefromList Actor)))
  (Default|CEReset (CallFunction|GetPiecefromList Actor)))

(fn ConstructionScript
  (|CallParentFunction))

(fn IsWatchedPiece
  (params (Actor :type Actor%20Object%20Reference))
  (return (Utilities|IsValid (CallFunction|GetPiecefromList Actor))))

(fn GetPiecefromList
  (params (Actor :type Actor%20Object%20Reference))
  (for _array_element (Variables|Default|GetPieceList)
    (if (== _array_element Actor)
      (return _array_element)))
  (return 0))