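; BP_RuinPiece is a grabbable physics piece in the Enigma1 folder that can be reset to its starting placement.
; The construction script applies the Mesh variable to the static mesh, and BeginPlay caches the actor transform.
; CE_Reset releases the piece from BPGrabComponent if held, fires its OnDropped dispatcher, restores the cached transform, and zeroes linear and angular velocity.
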(event Custom|CE_Reset
  (bind _staticmesh (Variables|Default|GetStaticMesh))
  (bind _bp_grabcomponent (Variables|Default|GetBP_GrabComponent))
  (if (Variables|/Game/_project/BP/Components/BP_GrabComponent.BP_GrabComponent_C|GetbIsHeld _bp_grabcomponent)
    (Default|TryRelease _bp_grabcomponent)
    (Default|CallOnDropped _bp_grabcomponent self))
  (Transformation|SetActorTransform (Variables|Default|GetDefaultTransform))
  (Physics|SetPhysicsLinearVelocity _staticmesh "0, 0, 0" false "None")
  (Class|PrimitiveComponent|SetPhysicsAngularVelocityinDegrees _staticmesh "0, 0, 0" false "None"))

(event EventBeginPlay
  (Variables|Default|SetDefaultTransform (Transformation|GetActorTransform)))

(fn ConstructionScript
  (Components|StaticMesh|SetStaticMesh (Variables|Default|GetStaticMesh) (Variables|Default|GetMesh)))