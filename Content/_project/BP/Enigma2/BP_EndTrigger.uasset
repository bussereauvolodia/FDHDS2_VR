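; End trigger actor for Enigma2 that holds a box volume and a target spot for a final puzzle piece.
; The construction script sizes the box and positions FinalEmplacement as an editor marker, which is destroyed on BeginPlay.
; SpawnFinalPiece teleports the existing Piece to the actor location plus the unrotated FinalPiecePlace offset, then prints a debug string.
; The file itself contains no overlap logic or call to SpawnFinalPiece.
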(event EventBeginPlay
  (Components|DestroyComponent (Variables|Default|GetFinal%20Emplacement)))

(event Collision|EventActorBeginOverlap
  (params (OtherActor :type Actor%20Object%20Reference)))

(event EventTick
  (params (DeltaSeconds :type Float%20%28single-precision%29)))

(fn ConstructionScript
  (Components|Box|SetBoxExtent (Variables|Default|GetBox) (Variables|Default|GetTriggerExtent) true)
  (Transformation|SetRelativeLocation (Variables|Default|GetFinal%20Emplacement) (Variables|Default|GetFinalPiecePlace) false false))

(fn GetFinalPiecePlace
  (return (+ (Variables|Default|GetFinalPiecePlace) (Transformation|GetActorLocation))))

(fn SpawnFinalPiece
  (Transformation|SetActorLocation (Variables|Default|GetPiece) (CallFunction|GetFinalPiecePlace) false true)
  (Development|PrintString "gugugaga"))