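; BP_RollingBall is a physics ball in Enigma2 that magnetically interacts with a BP_MagneticTablet.
; An attraction sphere tracks the overlapping tablet, and each tick applies an inverse-distance force to the tablet's mesh along the tablet-to-ball direction.
; Audio plays above a horizontal speed threshold, with volume scaled by squared speed.
; Reset teleports the ball to its starting transform, toggling physics around the move, and reacquires any overlapping tablet.
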(event OnComponentBeginOverlap(Sphere)
  (params (OverlappedComponent :type Primitive%20Component%20Object%20Reference) (OtherActor :type Actor%20Object%20Reference) (OtherComp :type Primitive%20Component%20Object%20Reference) (OtherBodyIndex :type Integer) (bFromSweep :type Boolean) (SweepResult :type Hit%20Result%20Structure%20%28by%20ref%29))
  (bind _asbp_magnetic_tablet (Utilities|Casting|CastToBP_MagneticTablet OtherActor))
  (Variables|Default|SetMagneticTablet _asbp_magnetic_tablet))

(event OnComponentEndOverlap(Sphere)
  (params (OverlappedComponent :type Primitive%20Component%20Object%20Reference) (OtherActor :type Actor%20Object%20Reference) (OtherComp :type Primitive%20Component%20Object%20Reference) (OtherBodyIndex :type Integer))
  (Utilities|Casting|CastToBP_MagneticTablet OtherActor)
  (Variables|Default|SetMagneticTablet 0))

(event Custom|CE_UpdateAudio
  (bind _returnvalue (Transformation|GetVelocity))
  (bind _audio (Variables|Default|GetAudio))
  (bind _returnvalue_2 (Class|KismetMathLibrary|VSizeXYSquared _returnvalue))
  (if (> _returnvalue_2 1e+02)
    (if (Variables|Default|GetIsPlayingSound)
      _
      (else
        (Audio|Components|Audio|Play _audio 0.0)
        (Variables|Default|SetIsPlayingSound true)))
    (Audio|Components|Audio|SetVolumeMultiplier _audio (/ _returnvalue_2 (Variables|Default|GetSoundMultiplierCoef)) :!class /Script/Engine.AudioComponent)
    (else
      (Audio|Components|Audio|Stop (Variables|Default|GetAudio))
      (Variables|Default|SetIsPlayingSound false))))

(event EventBeginPlay
  (Variables|Default|SetStartingPos (Transformation|GetActorTransform))
  (bind _asbp_magnetic_tablet (Utilities|Casting|CastToBP_MagneticTablet (Utilities|Array|Get(acopy) (Collision|GetOverlappingActors (Variables|Default|GetSphere) "/Game/_project/BP/Enigma2/BP_MagneticTablet.BP_MagneticTablet_C" :!class /Script/Engine.PrimitiveComponent))))
  (Variables|Default|SetMagneticTablet _asbp_magnetic_tablet))

(event EventTick
  (params (DeltaSeconds :type Float%20%28single-precision%29))
  (bind _returnvalue (Transformation|GetActorLocation))
  (bind _magnetictablet (Variables|Default|GetMagneticTablet))
  (bind _magnetictablet_2 (Variables|Default|GetMagneticTablet))
  (bind _returnvalue_2 (Transformation|GetActorLocation _magnetictablet_2))
  (bind _returnvalue_3 (- _returnvalue _returnvalue_2))
  (CallFunction|CEUpdateAudio)
  (Utilities|IsValid _magnetictablet
    (:Is%20Valid
      (Physics|AddForce (Variables|/Script/Engine.StaticMeshActor|GetStaticMeshComponent _magnetictablet) (* (Math|Vector|Normalize _returnvalue_3) (* (/ 2.0 (Math|Vector|VectorLength _returnvalue_3)) (Variables|Default|GetForceValue))) "None" false))))

(event EventReset
  (bind _sphere1 (Variables|Default|GetSphere1))
  (Physics|SetSimulatePhysics _sphere1 false)
  (Transformation|SetActorTransform (Variables|Default|GetStartingPos) false true)
  (Physics|SetSimulatePhysics _sphere1 true)
  (bind _asbp_magnetic_tablet (Utilities|Casting|CastToBP_MagneticTablet (Utilities|Array|Get(acopy) (Collision|GetOverlappingActors (Variables|Default|GetSphere) "/Game/_project/BP/Enigma2/BP_MagneticTablet.BP_MagneticTablet_C" :!class /Script/Engine.PrimitiveComponent))))
  (Variables|Default|SetMagneticTablet _asbp_magnetic_tablet))

(fn ConstructionScript
  (Components|Sphere|SetSphereRadius (Variables|Default|GetSphere) (Variables|Default|GetAttractionRadius) true))