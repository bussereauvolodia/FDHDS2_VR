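; Zone manager for the Enigma2 puzzle that resets puzzle pieces when they leave all of its zones.
; IsWatchedPiece treats any actor implementing IN_Resetable as a watched piece.
; On ActorLeftAllZones, it asks such an actor through ShouldResetMessage and calls ResetMessage on it if the answer is true.
; Zone tracking is not defined here, and BeginPlay, overlap and Tick are disabled stubs.
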(event EventBeginPlay
  (|CallParentFunction) ; This node is disabled and will not be called.\nDrag off pins to build functionality.
)

(event Collision|EventActorBeginOverlap
  (params (OtherActor :type Actor%20Object%20Reference)))

(event EventTick
  (params (DeltaSeconds :type Float%20%28single-precision%29)))

(event EventActorLeftAllZones
  (params (Actor :type Actor%20Object%20Reference))
  (if (Utilities|DoesObjectImplementInterface Actor "/Game/_project/Interface/IN_Resetable.IN_Resetable_C")
    (bind _state (Class|INResetable|ShouldReset(Message) Actor))
    (if _state
      (Class|INResetable|Reset(Message) Actor))))

(fn ConstructionScript
  (|CallParentFunction))

(fn IsWatchedPiece
  (params (Actor :type Actor%20Object%20Reference))
  (return (Utilities|DoesObjectImplementInterface Actor "/Game/_project/Interface/IN_Resetable.IN_Resetable_C")))