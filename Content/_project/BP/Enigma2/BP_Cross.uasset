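; BP_Cross is a physics-simulated cross prop in the Enigma2 folder, grabbable by motion controllers at a top and bottom grip.
; Each Tick it follows a single holding hand's transform, or with both hands sits at the top one and aims toward the bottom.
; Grabbing disables physics and clears the respawn timer.
; Full release restores physics and sets a timer for a delayed start-transform reset, but its zero time prevents firing.
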(event OnGrabbed(GrabCompTop)
  (params (MotionController :type Motion%20Controller%20Component%20Object%20Reference) (ActorGrabbed :type Actor%20Object%20Reference))
  (bind _respawnhandle (Variables|Default|GetRespawnHandle))
  (Variables|Default|SetTopGripController MotionController)
  (Physics|SetSimulatePhysics (Variables|Default|GetRoot) false)
  (if (Utilities|Time|IsValidTimerHandle _respawnhandle)
    (Utilities|Time|ClearandInvalidateTimerbyHandle _respawnhandle)))

(event OnGrabbed(GrabCompBot)
  (params (MotionController :type Motion%20Controller%20Component%20Object%20Reference) (ActorGrabbed :type Actor%20Object%20Reference))
  (bind _respawnhandle (Variables|Default|GetRespawnHandle))
  (Variables|Default|SetBottomGripController MotionController)
  (Physics|SetSimulatePhysics (Variables|Default|GetRoot) false)
  (if (Utilities|Time|IsValidTimerHandle _respawnhandle)
    (Utilities|Time|ClearandInvalidateTimerbyHandle _respawnhandle)))

(event OnDropped(GrabCompTop)
  (params (ActorDropped :type Actor%20Object%20Reference))
  (Variables|Default|SetTopGripController 0)
  (CallFunction|CheckifFullyDroppedandExec))

(event OnDropped(GrabCompBot)
  (params (ActorDropped :type Actor%20Object%20Reference))
  (Variables|Default|SetBottomGripController 0)
  (CallFunction|CheckifFullyDroppedandExec))

(event Custom|OnDropped
  ;[1 1 1] TODO: add drop timer reset stuff
  (Physics|SetSimulatePhysics (Variables|Default|GetRoot) true)
  (bind _returnvalue (Utilities|Time|SetTimerbyEvent (delegate Custom|RespawnDelayed) 0.0))
  (Variables|Default|SetRespawnHandle _returnvalue))

(event Custom|RespawnDelayed
  (Utilities|FlowControl|Delay (Variables|Default|GetRespawnDelay))
  (Transformation|SetActorTransform (Variables|Default|GetStartPos)))

(event EventBeginPlay
  (Physics|SetSimulatePhysics (Variables|Default|GetRoot) true)
  (Variables|Default|SetStartPos (Transformation|GetActorTransform)))

(event Collision|EventActorBeginOverlap
  (params (OtherActor :type Actor%20Object%20Reference)))

(event EventTick
  (params (DeltaSeconds :type Float%20%28single-precision%29))
  (bind _topgripcontroller (Variables|Default|GetTopGripController))
  (bind _bottomgripcontroller (Variables|Default|GetBottomGripController))
  (bind _topgripcontroller_2 (Variables|Default|GetTopGripController))
  (bind _topgripcontroller_3 (Variables|Default|GetTopGripController))
  (bind _bottomgripcontroller_2 (Variables|Default|GetBottomGripController))
  (bind _returnvalue (Utilities|IsValid _bottomgripcontroller_2))
  (bind _returnvalue_2 (Utilities|IsValid _topgripcontroller))
  (bind _returnvalue_3 (Transformation|GetWorldLocation _topgripcontroller_3))
  (bind _returnvalue_4 (select _returnvalue_2 _topgripcontroller_2 _bottomgripcontroller))
  (bind _returnvalue_5 (Transformation|GetWorldTransform _returnvalue_4))
  (if (and _returnvalue_2 _returnvalue)
    (Transformation|SetActorLocation _returnvalue_3 false false)
    (Transformation|SetActorRotation (Math|Rotator|MakeRotfromX (- (Transformation|GetWorldLocation (Variables|Default|GetBottomGripController)) _returnvalue_3)))
    (elif (or _returnvalue_2 _returnvalue)
      ;[1 1 1] TODO: Somehow snap to the hand maybe?
      (Transformation|SetActorRotation (.rotation _returnvalue_5))
      (Transformation|SetActorLocation (.location _returnvalue_5) false false))))

(fn ConstructionScript)

(fn CheckifFullyDroppedandExec
  (if (Math|Boolean|NORBoolean (Utilities|IsValid (Variables|Default|GetTopGripController)) (Utilities|IsValid (Variables|Default|GetBottomGripController)))
    (CallFunction|OnDropped)))