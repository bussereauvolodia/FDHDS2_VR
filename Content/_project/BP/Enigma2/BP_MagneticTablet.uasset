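; BP_MagneticTablet is a physics tablet in the Enigma2 puzzle that starts non-grabbable and can return to its starting position.
; BeginPlay disables BPGrab and stores the start transform, which Reset restores by teleporting with physics briefly switched off.
; Overlapping a BP_EndTrigger plays audio and logs arrival only if grabbing is already enabled, so setting CanBeGrabbed true there changes nothing.
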(event EventBeginPlay
  (Variables|/Game/_project/BP/Components/BP_GrabComponent.BP_GrabComponent_C|SetCanBeGrabbed (Variables|Default|GetBP_Grab) false)
  (Variables|Default|SetStartingPos (Transformation|GetActorTransform)))

(event Collision|EventActorBeginOverlap
  (params (OtherActor :type Actor%20Object%20Reference))
  (bind _bp_grab (Variables|Default|GetBP_Grab))
  (Utilities|Casting|CastToBP_EndTrigger OtherActor)
  (if (Variables|/Game/_project/BP/Components/BP_GrabComponent.BP_GrabComponent_C|GetCanBeGrabbed _bp_grab)
    (Variables|/Game/_project/BP/Components/BP_GrabComponent.BP_GrabComponent_C|SetCanBeGrabbed _bp_grab true)
    (Development|PrintString "Arrived at end trigger")
    (Audio|Components|Audio|Play (Variables|Default|GetAudio) 0.0)))

(event EventTick
  (params (DeltaSeconds :type Float%20%28single-precision%29)))

(event EventReset
  (bind _staticmeshcomponent (Variables|Default|GetStaticMeshComponent))
  (Physics|SetSimulatePhysics _staticmeshcomponent false)
  (Transformation|SetActorTransform (Variables|Default|GetStartingPos) false true)
  (Physics|SetSimulatePhysics _staticmeshcomponent true))

(fn ConstructionScript)