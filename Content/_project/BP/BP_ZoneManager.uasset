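; BP_ZoneManager tracks when watched actors leave a group of collision zones.
; On BeginPlay it assigns itself as manager to each zone in CollisionZones.
; ActorLeftZone checks the remaining zones for overlap and fires ActorLeftAllZones only when the watched actor is in none.
; IsWatchedPiece returns false and ActorLeftAllZones is empty, so as written the manager acts on nothing without overrides.
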(event Custom|ActorLeftZone
  (params (Actor :type Actor%20Object%20Reference))
  (if (CallFunction|IsWatchedPiece Actor)
    (bind _result (CallFunction|IsinZone Actor))
    (if (not _result)
      (CallFunction|ActorLeftAllZones Actor))))

(event Custom|ActorLeftAllZones
  (params (Actor :type Actor%20Object%20Reference)))

(event EventBeginPlay
  (for _array_element (Variables|Default|GetCollisionZones)
    (Variables|/Game/_project/BP/BP_CollisionZone.BP_CollisionZone_C|SetZoneManager _array_element self)))

(fn ConstructionScript)

(fn IsinZone
  (params (Actor :type Actor%20Object%20Reference))
  (for _array_element (Variables|Default|GetCollisionZones)
    (if (Default|IsActorOverlapping _array_element Actor)
      (return true)))
  (return false))

(fn IsWatchedPiece
  (params (Actor :type Actor%20Object%20Reference))
  (return false))