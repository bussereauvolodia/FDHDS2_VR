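; BP_NiagaraActivatorZone is a box trigger that switches a chosen Niagara system on or off for actors entering it.
; On begin overlap, it sends ChangeActivationOfSystemMessage to actors implementing IN_NiagaraHolder, passing NiagaraSystemToModify and the ActivateInZone state.
; On end overlap, it sends the inverse state rather than restoring the previous one.
; The receiving actor handles the actual activation through the interface.
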(event OnComponentBeginOverlap(Box)
  (params (OverlappedComponent :type Primitive%20Component%20Object%20Reference) (OtherActor :type Actor%20Object%20Reference) (OtherComp :type Primitive%20Component%20Object%20Reference) (OtherBodyIndex :type Integer) (bFromSweep :type Boolean) (SweepResult :type Hit%20Result%20Structure%20%28by%20ref%29))
  (if (Utilities|DoesObjectImplementInterface OtherActor "/Game/_project/Interface/IN_NiagaraHolder.IN_NiagaraHolder_C")
    (Class|INNiagaraHolder|ChangeActivationOfSystem(Message) OtherActor (Variables|Default|GetNiagaraSystemToModify) (Variables|Default|GetActivateInZone))))

(event OnComponentEndOverlap(Box)
  (params (OverlappedComponent :type Primitive%20Component%20Object%20Reference) (OtherActor :type Actor%20Object%20Reference) (OtherComp :type Primitive%20Component%20Object%20Reference) (OtherBodyIndex :type Integer))
  (if (Utilities|DoesObjectImplementInterface OtherActor "/Game/_project/Interface/IN_NiagaraHolder.IN_NiagaraHolder_C")
    (Class|INNiagaraHolder|ChangeActivationOfSystem(Message) OtherActor (Variables|Default|GetNiagaraSystemToModify) (not (Variables|Default|GetActivateInZone)))))

(fn ConstructionScript)