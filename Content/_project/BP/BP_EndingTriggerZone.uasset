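; BP_EndingTriggerZone is a trigger volume that starts the game's ending and shows the outro credits.
; A widget component stays hidden from BeginPlay until the player character first overlaps the box.
; That overlap calls OnEndingStart, sets a one-shot flag, reveals the widget and plays the credits on its WB_Outro_Credits instance.
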(event OnComponentBeginOverlap(Box)
  (params (OverlappedComponent :type Primitive%20Component%20Object%20Reference) (OtherActor :type Actor%20Object%20Reference) (OtherComp :type Primitive%20Component%20Object%20Reference) (OtherBodyIndex :type Integer) (bFromSweep :type Boolean) (SweepResult :type Hit%20Result%20Structure%20%28by%20ref%29))
  (bind _widget (Variables|Default|GetWidget))
  (if (and (== OtherActor (Game|GetPlayerCharacter 0)) (not (Variables|Default|GetHasPlayedEnd)))
    (Default|CallOnEndingStart)
    (Variables|Default|SetHasPlayedEnd true)
    (Development|SetHiddeninGame _widget false false)
    (bind _aswb_outro_credits (Utilities|Casting|CastToWB_Outro_Credits (UserInterface|GetWidget _widget)))
    (Default|CEPlayCredits _aswb_outro_credits)))

(event EventBeginPlay
  (Development|SetHiddeninGame (Variables|Default|GetWidget) true false))

(fn ConstructionScript)