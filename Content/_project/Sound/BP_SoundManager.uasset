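; Sound manager actor that plays the game's sound effects and music through two audio components, SFX and Music.
; PlaySFX and PlayMusic each swap the given sound into their component and play it from the start, so each channel holds one sound at a time.
; SetVolume applies a single volume multiplier to both components at once.
; The event graph and construction script are empty.
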(event EventBeginPlay)

(event Collision|EventActorBeginOverlap
  (params (OtherActor :type Actor%20Object%20Reference)))

(event EventTick
  (params (DeltaSeconds :type Float%20%28single-precision%29)))

(fn ConstructionScript)

(fn PlaySFX
  (params (Sound :type Sound%20Base%20Object%20Reference))
  (bind _sfx (Variables|Default|GetSFX))
  (Audio|Components|Audio|SetSound _sfx Sound)
  (Audio|Components|Audio|Play _sfx 0.0))

(fn PlayMusic
  (params (Sound :type Sound%20Base%20Object%20Reference))
  (bind _music (Variables|Default|GetMusic))
  (Audio|Components|Audio|SetSound _music Sound)
  (Audio|Components|Audio|Play _music 0.0))

(fn SetVolume
  (params (NewVolumeMultiplier :type Float%20%28single-precision%29))
  (Audio|Components|Audio|SetVolumeMultiplier (Variables|Default|GetSFX) NewVolumeMultiplier :!class /Script/Engine.AudioComponent)
  (Audio|Components|Audio|SetVolumeMultiplier (Variables|Default|GetMusic) NewVolumeMultiplier :!class /Script/Engine.AudioComponent))